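; Medical number slide that displays an integer on a text render component and hides it while the number changes.
; SetValue stores a pending value and calls Hide if the slide is visible, otherwise it runs the update directly.
; VisibleChanged swaps the text while hidden, calls Show, then commits the value once visible.
; A negative value is committed without showing, so the slide stays hidden.
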(event `self.VisibleChanged`
  (params (Visible :type Boolean))
  (bind _new_value (`self.New Value`))
  (if Visible
    (set `self.Value` (`self.New Value`))
    (elif (!= (`self.Value`) _new_value)
      (if (>= _new_value 0)
        (`TextRenderComponent.K2_SetText` (`self.TextRender`) (`KismetTextLibrary.Conv_IntToText` _new_value))
        (`self.Show`)
        (else
          (set `self.Value` (`self.New Value`)))))))

(fn `SetValue`
  (params (Value :type Integer))
  (if (and (!= Value (`self.Value`)) (!= (`self.New Value`) Value))
    (set `self.New Value` Value)
    (if (`self.Visible`)
      (`self.Hide`)
      (else
        (`self.VisibleChanged` false)))))

(fn `UserConstructionScript`
  (`parent.UserConstructionScript`))