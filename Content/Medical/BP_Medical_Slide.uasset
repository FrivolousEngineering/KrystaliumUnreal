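; BP_Medical_Slide is an actor that slides a Slide component in and out along local Y and swaps its material while hidden.
; Tick advances or rewinds T at a set Speed, mapping it through a float curve to a position between Minimum and Maximum.
; SetMaterial queues a new material and hides the slide; once hidden, VisibleChanged applies it and calls Show to slide it back in.
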(event `self.ReceiveBeginPlay`)

(event `self.ReceiveTick`
  (params (DeltaSeconds :type "Float (single-precision)"))
  (bind _t (`self.t`))
  (bind _t_2 (`self.t`))
  (if (`self.Visible`)
    ;[1 1 1] Visible
    (if (< _t 1.0)
      (bind _output_get (set `self.t` (+ _t (* (`self.Speed`) DeltaSeconds))))
      (`self.SetYPositionFromCurve` (`self.Minimum`) (`self.Maximum`) _output_get (`self.Curve`) (`self.Slide`))
      (if (>= (`self.t`) 1.0)
        (`self.VisibleChanged` true)))
    (else
      ;[1 1 1] Not Visible
      (if (> _t_2 0.0)
        (bind _output_get_2 (set `self.t` (- _t_2 (* (`self.Speed`) DeltaSeconds))))
        (`self.SetYPositionFromCurve` (`self.Minimum`) (`self.Maximum`) _output_get_2 (`self.Curve`) (`self.Slide`))
        (if (<= (`self.t`) 0.0)
          (`self.VisibleChanged` false))))))

(event `VisibleChanged`
  (params (Visible :type Boolean))
  (if Visible
    (set `self.Material` (`self.NewMaterial`))
    (elif (!= (`self.Material`) (`self.NewMaterial`))
      (`PrimitiveComponent.SetMaterial` (`self.Slide`) 0 (`self.NewMaterial`))
      (`self.Show`))))

(fn `Hide`
  (if (`self.Visible`)
    (set `self.Visible` false)
    (`SceneComponent.K2_SetRelativeLocation` (`self.Slide`) (`KismetMathLibrary.MakeVector` 0.0 (`self.Maximum`)) false false)
    (set `self.t` 1.0)
    (else
      (return))))

(fn `SetMaterial`
  (params (Material :type "MaterialInterface Object Reference"))
  (if (and (!= Material (`self.Material`)) (!= Material (`self.NewMaterial`)))
    (set `self.NewMaterial` Material)
    (if (`self.Visible`)
      (`self.Hide`)
      (else
        (`self.VisibleChanged` false)))))

(fn `SetYPositionFromCurve`
  (params (Minimum :type "Float (double-precision)") (Maximum :type "Float (double-precision)") (Time :type "Float (double-precision)") (Curve :type "CurveFloat Object Reference") (Target :type "SceneComponent Object Reference"))
  (`SceneComponent.K2_SetRelativeLocation` Target (`KismetMathLibrary.MakeVector` 0.0 (`KismetMathLibrary.Lerp` Minimum Maximum (`CurveFloat.GetFloatValue` Curve Time))) false false))

(fn `Show`
  (if (`self.Visible`)
    (return)
    (else
      (set `self.Visible` true)
      (`SceneComponent.K2_SetRelativeLocation` (`self.Slide`) (`KismetMathLibrary.MakeVector` 0.0 (`self.Minimum`)) false false)
      (set `self.t` 0.0))))

(fn `UserConstructionScript`)