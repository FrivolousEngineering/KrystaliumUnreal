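; BP_Medical_MessageSlide is a medical message slide that displays text on a TextRender and swaps messages through hide and show transitions.
; SetText stores a changed message as pending, then hides the slide, or updates it immediately if already hidden.
; VisibleChanged writes pending text while hidden and shows the slide again, then commits it as current once visible, so text changes only out of view.
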(event `self.ReceiveTick`
  (params (DeltaSeconds :type "Float (single-precision)"))
  (`parent.ReceiveTick` DeltaSeconds))

(event `self.VisibleChanged`
  (params (Visible :type Boolean))
  (bind _newtext (`self.NewText`))
  (if Visible
    (set `self.Text` (`self.NewText`))
    (elif (`KismetStringLibrary.NotEqual_StrStr` (`self.Text`) _newtext)
      (`TextRenderComponent.K2_SetText` (`self.TextRender`) (`KismetTextLibrary.Conv_StringToText` _newtext))
      (`self.Show`))))

(fn `SetText`
  (params (Text :type String))
  (if (and (`KismetStringLibrary.NotEqual_StrStr` Text (`self.Text`)) (`KismetStringLibrary.NotEqual_StrStr` Text (`self.NewText`)))
    (set `self.NewText` Text)
    (if (`self.Visible`)
      (`self.Hide`)
      (else
        (`self.VisibleChanged` false)))))

(fn `UserConstructionScript`
  (`parent.UserConstructionScript`))