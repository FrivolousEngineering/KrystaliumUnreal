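; BP_Controller is a medical code-entry controller that collects up to five numbers and broadcasts changes, messages, valid input and resets through event dispatchers.
; Keys filtered by a valid-number list append digits, Backspace removes one, and letter shortcuts trigger invalid, valid, reset, clear and "Awaiting Sample" states.
; Entry and validation functions set a timeout, but its countdown logic and the InvalidInput dispatch are disconnected.
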(event `self.ReceiveTick`
  (params (DeltaSeconds :type "Float (single-precision)")))

(event `Key|AnyKey`
  (params (Key :type "Key Structure"))
  (bind _returnvalue (`KismetTextLibrary.Conv_TextToString` (`KismetInputLibrary.Key_GetDisplayName` Key)))
  (:`Pressed`
    (if (`BlueprintSetLibrary.Set_Contains` (`self.Valid Nuimbers`) _returnvalue)
      (`self.AppendNumber` (`KismetStringLibrary.Conv_StringToInt` _returnvalue)))))

(event `Key|BackSpace`
  (params (Key :type "Key Structure"))
  (:`Pressed`
    (`self.RemoveLastNumber`)))

(event `Key|I`
  (params (Key :type "Key Structure"))
  (:`Pressed`
    (`self.Invalid`)))

(event `Key|V`
  (params (Key :type "Key Structure"))
  (:`Pressed`
    (`self.Valid`)))

(event `Key|R`
  (params (Key :type "Key Structure"))
  (:`Pressed`
    (`self.Reset`)))

(event `Key|C`
  (params (Key :type "Key Structure"))
  (:`Pressed`
    (`self.ClearNumbers`)
    (`self.Message` "Enter Code:")))

(event `Key|S`
  (params (Key :type "Key Structure"))
  (:`Pressed`
    (`self.Message` "Awaiting Sample")))

(fn `AppendNumber`
  (params (Number :type Integer))
  (if (< (`KismetArrayLibrary.Array_Length` (`self.Numbers`)) 5)
    (`KismetArrayLibrary.Array_Add` (`self.Numbers`) Number)
    (set `self.Timer` 10.0)
    (`self.NumbersChanged`)))

(fn `ClearNumbers`
  (`KismetArrayLibrary.Array_Clear` (`self.Numbers`))
  (`self.NumbersChanged`))

(fn `Invalid`
  (set `self.Timer` 5.0)
  (`self.ShowMessage` "Invalid Input!"))

(fn `Message`
  (params (Message :type String))
  (`self.ShowMessage` Message))

(fn `RemoveLastNumber`
  (bind _numbers (`self.Numbers`))
  (if (`KismetArrayLibrary.Array_IsNotEmpty` (`self.Numbers`))
    (`KismetArrayLibrary.Array_Remove` _numbers (`KismetArrayLibrary.Array_LastIndex` _numbers))
    (set `self.Timer` 10.0)
    (`self.NumbersChanged`)))

(fn `Reset`
  (`self.ClearNumbers`)
  (`self.ControllerReset`))

(fn `SetNumbers`
  (params (Numbers :type "Array of Integer"))
  (set `self.Numbers` Numbers)
  (`self.NumbersChanged`))

(fn `UserConstructionScript`)

(fn `Valid`
  (set `self.Timer` 0.0)
  (`self.ValidInput`))